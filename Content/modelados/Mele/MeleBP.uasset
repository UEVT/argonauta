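; MeleBP is a melee enemy that chases and attacks the VR player.
; PawnSensing drives AIMoveTo until in range, then it stops, faces the player and deals delayed damage with haptics on both controllers, without rechecking range.
; Tagged bullet and sword overlaps subtract health, followed by a brief invulnerability window.
; Tick destroys it at zero health or updates a health-bar widget yawed toward the player.
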(event OnSeePawn(PawnSensing)
  (params (Pawn :type Pawn%20Object%20Reference))
  ;[1 1 1] IA(por mejorar)
  (bind _asvrpawn (Utilities|Casting|CastToVRPawn Pawn))
  (if (<= (Math|Vector|Distance(Vector) (Transformation|GetActorLocation _asvrpawn) (Transformation|GetActorLocation)) 2e+02)
    (Class|NavMovementComponent|StopActiveMovement (Variables|Character|GetCharacterMovement))
    (Transformation|SetActorRotation (Math|Rotator|MakeRotator 0.0 0.0 (.Yaw (Math|Rotator|BreakRotator (Math|Rotator|FindLookatRotation (Transformation|GetActorLocation) (Transformation|GetActorLocation (Game|GetPlayerCharacter 0)))))))
    (CallFunction|Atacar)
    (else
      (AI|AIMoveTo self "0, 0, 0" _asvrpawn 5.0 false))))

(event Custom|BalaUsg
  ;[1 1 1] Daño bala USG
  (Variables|Default|Setdañable false)
  (Variables|Default|SetLifeBar (- (Variables|Default|GetLifeBar) 7.0))
  (Utilities|FlowControl|Delay 0.5)
  (Variables|Default|Setdañable true))

(event Custom|bala
  ;[1 1 1] Daño bala
  (Variables|Default|Setdañable false)
  (Variables|Default|SetLifeBar (- (Variables|Default|GetLifeBar) 15.0))
  (Utilities|FlowControl|Delay 0.5)
  (Variables|Default|Setdañable true))

(event Custom|Espada2
  ;[1 1 1] Daño espada 2
  (Variables|Default|Setdañable false)
  (Variables|Default|SetLifeBar (- (Variables|Default|GetLifeBar) 55.0))
  (Utilities|FlowControl|Delay 0.5)
  (Variables|Default|Setdañable true))

(event Custom|espada
  ;[1 1 1] Daño espada
  (Variables|Default|Setdañable false)
  (Variables|Default|SetLifeBar (- (Variables|Default|GetLifeBar) 35.0))
  (Utilities|FlowControl|Delay 0.5)
  (Variables|Default|Setdañable true))

(event Custom|Atacar
  (bind _returnvalue (Game|GetPlayerController 0))
  (if (Variables|Default|GetCAttack)
    (Variables|Default|SetCAttack false)
    (bind _asvrpawn (Utilities|Casting|CastToVRPawn (Game|Player|GetPlayerPawn 0)))
    (Utilities|FlowControl|Delay 1.0)
    (Variables|/Game/VRTemplate/Blueprints/VRPawn.VRPawn_C|SetViadaPlayer _asvrpawn (- (Variables|/Game/VRTemplate/Blueprints/VRPawn.VRPawn_C|GetViadaPlayer _asvrpawn) 15.0))
    (Class|PlayerController|PlayHapticEffect _returnvalue "/Game/VRTemplate/Haptics/GrabHapticEffect.GrabHapticEffect" "Left" 1.0 false)
    (Class|PlayerController|PlayHapticEffect _returnvalue "/Game/VRTemplate/Haptics/GrabHapticEffect.GrabHapticEffect" "Right" 1.0 false)
    (Utilities|FlowControl|Delay 0.5)
    (Variables|Default|SetCAttack true)))

(event EventBeginPlay)

(event EventTick
  (params (DeltaSeconds :type Float%20%28single-precision%29))
  ;[1 1 1] Sistema de vida
  (if (<= (Variables|Default|GetLifeBar) 0.0)
    (Actor|DestroyActor)
    (else
      (bind _asestado_e (Utilities|Casting|CastToEstadoE (UserInterface|GetUserWidgetObject (Variables|Default|Getvida))))
      (Progress|SetPercent (Variables|/Game/modelados/Enemy/EstadoE.EstadoE_C|GetProgressBar_0 _asestado_e) (/ (Variables|Default|GetLifeBar) 1e+02))
      (Transformation|SetWorldRotation (Variables|Default|Getvida) (Math|Rotator|MakeRotator 0.0 0.0 (.Yaw (Math|Rotator|BreakRotator (Math|Rotator|FindLookatRotation (Transformation|GetWorldLocation (Variables|Default|Getvida)) (Transformation|GetActorLocation (Game|GetPlayerCharacter 0)))))) false false))))

(event Collision|EventActorBeginOverlap
  (params (OtherActor :type Actor%20Object%20Reference))
  ;[1 1 1] Sistema de daño
  (if (Math|Boolean|Equal(Boolean) (Variables|Default|Getdañable) true)
    (if (Actor|ActorHasTag OtherActor "Bala")
      (CallFunction|Bala)
      (elif (Actor|ActorHasTag OtherActor "Espada1")
        (CallFunction|Espada)
        (elif (Actor|ActorHasTag OtherActor "BalaUSG")
          (CallFunction|BalaUsg)
          (elif (Actor|ActorHasTag OtherActor "Espada2")
            (CallFunction|Espada2)))))))

(fn ConstructionScript)